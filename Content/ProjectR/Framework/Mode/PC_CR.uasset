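; PC_CR is a player controller that links the controlled IsometricPlayer pawn to the controller and puts the WBP_CR widget on screen.
; On BeginPlay it sets the deprecated input yaw scale, then caches the pawn in CharRef and hands it a back-reference to itself.
; It also creates the widget, stores it and adds it to the viewport, with validity checks guarding both setups.
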(event EventBeginPlay
  (Class|PlayerController|SetDeprecatedInputYawScale 1.0)
  (Utilities|FlowControl|Sequence
    (:then_0
      (Variables|Refs|GetCharRef
        (:then)
        (:else
          (bind _asisometric_player (Utilities|Casting|CastToIsometricPlayer (Pawn|GetControlledPawn)))
          (bind _output_get (Variables|Refs|SetCharRef _asisometric_player))
          (Variables|/Game/ProjectR/IsometricPlayer/IsometricPlayer.IsometricPlayer_C|SetPC_Ref _output_get self))))
    (:then_1
      (Variables|Refs|GetWBP_Ref
        (:then)
        (:else
          (bind _returnvalue (UserInterface|CreateWidget "/Game/ProjectR/UI/WBP_CR.WBP_CR_C" self))
          (bind _output_get_2 (Variables|Refs|SetWBP_Ref _returnvalue))
          (UserInterface|Viewport|AddtoViewport _output_get_2 0))))))

(event EventTick
  (params (DeltaSeconds :type Float%20%28single-precision%29)))

(fn ConstructionScript)