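; Bot enemy actor that tints its Manny mesh and tags itself as an enemy.
; The construction script creates dynamic material instances for both mesh material slots, tinting one dark purple and the other red.
; On BeginPlay it adds replicated loose gameplay tags for enemy type and idle state, and replaces its actor Tags with "Enemy".
; No AI or combat logic lives in these graphs.
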(event EventBeginPlay
  (|AddEnemyGTag))

(event Collision|EventActorBeginOverlap
  (params (OtherActor :type Actor%20Object%20Reference)))

(event EventTick
  (params (DeltaSeconds :type Float%20%28single-precision%29)))

(fn ConstructionScript
  (bind _mesh (Variables|Character|GetMesh))
  (Utilities|FlowControl|Sequence
    (:then_0
      (bind _returnvalue (Rendering|Material|CreateDynamicMaterialInstance _mesh 0 "/Game/Characters/Mannequins/Materials/Instances/Manny/MI_Manny_01.MI_Manny_01" "None" :!class /Script/Engine.PrimitiveComponent))
      (Rendering|Material|SetMaterial _mesh 0 _returnvalue)
      (Rendering|Material|SetVectorParameterValue _returnvalue "Tint" "(R=0.100000,G=0.000000,B=0.150000,A=1.000000)" :!class /Script/Engine.MaterialInstanceDynamic))
    (:then_1
      (bind _returnvalue_2 (Rendering|Material|CreateDynamicMaterialInstance _mesh 1 "/Game/Characters/Mannequins/Materials/Instances/Manny/MI_Manny_02.MI_Manny_02" "None" :!class /Script/Engine.PrimitiveComponent))
      (Rendering|Material|SetMaterial _mesh 1 _returnvalue_2)
      (Rendering|Material|SetVectorParameterValue _returnvalue_2 "Tint" "(R=1.000000,G=0.000000,B=0.000000,A=1.000000)" :!class /Script/Engine.MaterialInstanceDynamic))))