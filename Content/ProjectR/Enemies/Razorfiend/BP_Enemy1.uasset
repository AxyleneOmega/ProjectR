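; Enemy Blueprint for the Razorfiend that tags itself as an enemy and carries a spline-driven attack movement.
; On BeginPlay it adds a replicated loose gameplay tag and sets its actor tags to Enemy.
; The AtkTimline event plays a timeline that moves the actor along its spline without sweeping.
; The nodes that detach the spline, scale the play rate by AtkTime and bind that event are disconnected.
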(event Custom|AtkTimline
  (bind _spline (Variables|Default|GetSpline))
  ;[1 1 1] Comment
  (bind _newtrack_0 (Timeline|Timeline PlayFromStart)
    (:Update
      (Transformation|SetActorLocation (Spline|GetLocationatDistanceAlongSpline _spline (Math|Float|Lerp 0.0 (Spline|GetSplineLength _spline) _newtrack_0) "World") false false))))

(event EventBeginPlay
  ;[1 1 1] Comment
  (|AddEnemyGTag))

(fn ConstructionScript)