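; BoltBreaker enemy actor that starts a damage component, tags itself as an enemy and deals melee damage with its hammer.
; Hammer overlaps send complex damage and hit data to the other actor's damage component, fetched through an interface call.
; Death spawns an explosion and destroys the actor after a short delay.
; Events toggle a weapon trail, Tick prints debug health, and most other interface functions are stubs.
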(event OnComponentBeginOverlap(hammur)
  (params (OverlappedComponent :type Primitive%20Component%20Object%20Reference) (OtherActor :type Actor%20Object%20Reference) (OtherComp :type Primitive%20Component%20Object%20Reference) (OtherBodyIndex :type Integer) (bFromSweep :type Boolean) (SweepResult :type Hit%20Result%20Structure%20%28by%20ref%29))
  (bind (_bblockinghit _binitialoverlap _time _distance _location _impactpoint _normal _impactnormal _physmat _hitactor _hitcomponent _hitbonename) (Collision|BreakHitResult SweepResult))
  (if (!= OtherActor self)
    (bind _bpc_dc (Class|BPIPawn|DCGetDamageComponent(Message) OtherActor))
    (Class|BPIDamage|ExecuteComplexDamage(Message) _bpc_dc "/Game/ProjectR/Systems/DamageSystem/ClassDamage/ChildDamageClasses/CD_Melee.CD_Melee_C" 75.0 self (Utilities|Struct|MakeS_HitData _bblockinghit _location _impactpoint _normal _impactnormal _hitactor _hitcomponent _hitbonename))))

(event OnDeath(BPC_DamageComponent)
  (bind _returnvalue (Transformation|GetActorTransform))
  (Niagara|SpawnSystematLocation "/Game/ProjectR/Assets/Particles/AdvancedMagicFX13/Particles/Niagara/NS_ky_explosion1.NS_ky_explosion1" (.location _returnvalue) (.rotation _returnvalue) (.scale _returnvalue) true true "AutoRelease")
  (Utilities|FlowControl|Delay 0.2)
  (Actor|DestroyActor))

(event Custom|StartTrail
  (Effects|Particles|Trails|BeginTrails (Variables|Default|GetTrail) "StartTrail" "EndTrail" "ETrailWidthMode_FromCentre" 1.0))

(event Custom|EndTrail
  (Effects|Particles|Trails|EndTrails (Variables|Default|GetTrail)))

(event EventTick
  (params (DeltaSeconds :type Float%20%28single-precision%29))
  (bind _currenthealth (Class|BPIDamage|GetCurrentHealth(Message) (Variables|Default|GetBPC_DamageComponent)))
  (Development|PrintString (Utilities|String|Append "BoltBreaker Health : " (Utilities|String|ToString(Float) _currenthealth)) true true "(R=1.000000,G=0.080507,B=0.000000,A=1.000000)" DeltaSeconds))

(event EventBeginPlay
  (|AddEnemyGTag)
  (Default|StartSystem (Variables|Default|GetBPC_DamageComponent) 1e+03))

(fn ConstructionScript)

(fn ACGetAttackComponent
  (return 0))

(fn AimGetRawAimDir
  (return "0, 0, 0"))

(fn ConfigCameraLag
  (params (CameraLagParams :type F%20Camera%20Lag%20Params%20Structure) (Interpolate? :type Boolean) (InterpTime :type Float%20%28double-precision%29))
  (return false))

(fn DCGetDamageComponent
  (return (Variables|Default|GetBPC_DamageComponent)))

(fn GetActionState
  (return "NewEnumerator0"))

(fn GetCMC
  (return 0))

(fn GetMeshForwardVector
  (return "0, 0, 0"))

(fn GetResolvedTargetDirection
  (return "0, 0, 0"))

(fn GetUsingUpperBodyAnim
  (return false 0 "NewEnumerator0"))

(fn GetViewRelativeRotation
  (return "0, 0, 0"))

(fn ResetCameraLag
  (params (Interpolate? :type Boolean) (InterpTime :type Float%20%28double-precision%29) (EaseExponent :type Float%20%28double-precision%29))
  (return false))

(fn UpdatePromptText
  (params (PromptText :type String))
  (return false))