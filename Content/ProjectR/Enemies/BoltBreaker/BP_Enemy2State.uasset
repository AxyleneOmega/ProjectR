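; BoltBreaker enemy actor that uses a StateTree, a damage component and gameplay tags marking it as an idle enemy.
; The player entering its sphere sends a one-time Alerted StateTree event.
; Hammer overlaps deal melee damage through the other actor's damage component, while its own health changes update a widget bar.
; Death spawns an explosion before destroying it; Tick prints debug health, and most interface functions are empty stubs.
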(event OnComponentBeginOverlap(hammur)
  (params (OverlappedComponent :type Primitive%20Component%20Object%20Reference) (OtherActor :type Actor%20Object%20Reference) (OtherComp :type Primitive%20Component%20Object%20Reference) (OtherBodyIndex :type Integer) (bFromSweep :type Boolean) (SweepResult :type Hit%20Result%20Structure%20%28by%20ref%29))
  (bind (_bblockinghit _binitialoverlap _time _distance _location _impactpoint _normal _impactnormal _physmat _hitactor _hitcomponent _hitbonename) (Collision|BreakHitResult SweepResult))
  (if (!= OtherActor self)
    (bind _bpc_dc (Class|BPIPawn|DCGetDamageComponent(Message) OtherActor))
    (Class|BPIDamage|ExecuteComplexDamage(Message) _bpc_dc "/Game/ProjectR/Systems/DamageSystem/ClassDamage/ChildDamageClasses/CD_Melee.CD_Melee_C" 75.0 self (Utilities|Struct|MakeS_HitData _bblockinghit _location _impactpoint _normal _impactnormal _hitactor _hitcomponent _hitbonename))))

(event OnDeath(BPC_DamageComponent)
  (bind _returnvalue (Transformation|GetActorTransform))
  (Niagara|SpawnSystematLocation "/Game/ProjectR/Assets/Particles/AdvancedMagicFX13/Particles/Niagara/NS_ky_explosion1.NS_ky_explosion1" (.location _returnvalue) (.rotation _returnvalue) (.scale _returnvalue) true true "AutoRelease")
  (Utilities|FlowControl|Delay 0.2)
  (Actor|DestroyActor))

(event OnComponentBeginOverlap(Sphere)
  (params (OverlappedComponent :type Primitive%20Component%20Object%20Reference) (OtherActor :type Actor%20Object%20Reference) (OtherComp :type Primitive%20Component%20Object%20Reference) (OtherBodyIndex :type Integer) (bFromSweep :type Boolean) (SweepResult :type Hit%20Result%20Structure%20%28by%20ref%29))
  ;[1 1 1] Comment
  (if (and (== (Game|GetPlayerCharacter 0) OtherActor) (not (GameplayTags|HasTag (Variables|Default|GetTag%20State%20Container) "(TagName=\"StateTree.Alerted\")" true)))
    (Gameplay|StateTree|SendStateTreeEvent (Variables|Default|GetStateTree) (Utilities|Struct|MakeStateTreeEvent "(TagName=\"StateTree.Alerted\")" "Enemy alert") :!class /Script/GameplayStateTreeModule.StateTreeComponent)
    (GameplayTags|AddGameplayTag (Variables|Default|GetTag%20State%20Container) "(TagName=\"StateTree.Alerted\")" :!class /Script/GameplayTags.BlueprintGameplayTagLibrary)))

(event Custom|OnEnemyHealthChange
  (params (Change :type Float%20%28double-precision%29))
  (bind _currenthealthpercent (Class|BPIDamage|GetHealthPercent(Message) (Variables|Default|GetBPC_DamageComponent)))
  (Class|BPIEnemyUI|UpdateEnemyHealthBar(Message) (UserInterface|GetUserWidgetObject (Variables|Default|GetWidget)) Change _currenthealthpercent))

(event EventTick
  (params (DeltaSeconds :type Float%20%28single-precision%29))
  (bind _currenthealth (Class|BPIDamage|GetCurrentHealth(Message) (Variables|Default|GetBPC_DamageComponent)))
  (Development|PrintString (Utilities|String|Append "BoltBreaker Health : " (Utilities|String|ToString(Float) _currenthealth)) true true "(R=1.000000,G=0.080507,B=0.000000,A=1.000000)" DeltaSeconds))

(event EventBeginPlay
  (|AddEnemyGTag_2)
  (Default|StartSystem (Variables|Default|GetBPC_DamageComponent) 1e+03)
  (EventDispatchers|BindEventtoOnHealthChange (Variables|Default|GetBPC_DamageComponent) (delegate Custom|OnEnemyHealthChange))
  (CallFunction|OnEnemyHealthChange 0.0))

(fn ConstructionScript)

(fn SetAtkTagContainer
  (params (AtkTagContainer :type Gameplay%20Tag%20Container%20Structure))
  (Variables|Default|SetAtk%20Tag%20Container AtkTagContainer))

(fn ACGetAttackComponent
  (return 0))

(fn AimGetRawAimDir
  (return "0, 0, 0"))

(fn ConfigCameraLag
  (params (CameraLagParams :type F%20Camera%20Lag%20Params%20Structure) (Interpolate? :type Boolean) (InterpTime :type Float%20%28double-precision%29))
  (return false))

(fn DCGetDamageComponent
  (return (Variables|Default|GetBPC_DamageComponent)))

(fn GetActionState
  (return "NewEnumerator0"))

(fn GetCMC
  (return 0))

(fn GetMeshForwardVector
  (return "0, 0, 0"))

(fn GetResolvedTargetDirection
  (return "0, 0, 0"))

(fn GetUsingUpperBodyAnim
  (return false 0 "NewEnumerator0"))

(fn GetViewRelativeRotation
  (return "0, 0, 0"))

(fn ResetCameraLag
  (params (Interpolate? :type Boolean) (InterpTime :type Float%20%28double-precision%29) (EaseExponent :type Float%20%28double-precision%29))
  (return false))

(fn UpdatePromptText
  (params (PromptText :type String))
  (return false))