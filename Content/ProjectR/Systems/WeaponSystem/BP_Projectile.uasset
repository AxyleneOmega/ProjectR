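; Data-driven weapon projectile that turns into an area-of-effect damage volume on impact.
; ProjectileData configures movement at construction, then mesh, scale and lifespan at BeginPlay.
; An overlap whose swept hit component blocks GameTraceChannel3 swaps the same mesh component to ColliderData's mesh, scale and the Aoe collision profile.
; Later overlaps send complex damage messages with ColliderData's damage and the hit details; hit and overlap events also print debug names.
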(event OnComponentBeginOverlap(StaticMesh)
  (params (OverlappedComponent :type Primitive%20Component%20Object%20Reference) (OtherActor :type Actor%20Object%20Reference) (OtherComp :type Primitive%20Component%20Object%20Reference) (OtherBodyIndex :type Integer) (bFromSweep :type Boolean) (SweepResult :type Hit%20Result%20Structure%20%28by%20ref%29))
  (bind (_bblockinghit _binitialoverlap _time _distance _location _impactpoint _normal _impactnormal _physmat _hitactor _hitcomponent _hitbonename) (Collision|BreakHitResult SweepResult))
  (bind _colliderdata (Variables|InitVars|GetColliderData))
  (bind _colliderdata_2 (Variables|InitVars|GetColliderData))
  (bind (_collidersm _colliderrelativetransform) (Utilities|Struct|BreakS_DamageColliderData _colliderdata))
  (bind (_damageclass _rawdamage) (Utilities|Struct|BreakS_DamageColliderData _colliderdata_2))
  (Development|PrintString (Utilities|GetDisplayName OtherComp))
  (if (Variables|Default|GetbAOEActivated)
    (Class|IDamage|ExecuteComplexDamage(Message) OtherActor (Utilities|ResolveSoftReference _damageclass) _rawdamage (Components|GetOwner) (Utilities|Struct|MakeS_HitData _bblockinghit _location _impactpoint _normal _impactnormal _hitactor _hitcomponent _hitbonename))
    (else
      (switch Utilities|FlowControl|Switch|SwitchonECollisionResponse (Collision|GetCollisionResponsetoChannel _hitcomponent "ECC_GameTraceChannel3")
        (:ECR_Block
          (Variables|Default|SetbAOEActivated true)
          (Utilities|SetStaticMesh _collidersm (Math|Transform|MakeTransform "0, 0, 0" "0, 0, 0" (.scale _colliderrelativetransform)))
          (Collision|SetCollisionProfileName (Variables|Default|GetStaticMesh) "Aoe" true :!class /Script/Engine.PrimitiveComponent))))))

(event EventBeginPlay
  (bind _projectiledata (Variables|InitVars|GetProjectileData))
  (bind (_lifespan _projectile_sm _projectilert) (Utilities|Struct|BreakS_Projectile _projectiledata))
  (Utilities|SetStaticMesh _projectile_sm _projectilert)
  (Actor|SetLifeSpan self _lifespan))

(event Collision|EventHit
  (params (MyComp :type Primitive%20Component%20Object%20Reference) (Other :type Actor%20Object%20Reference) (OtherComp :type Primitive%20Component%20Object%20Reference) (bSelfMoved :type Boolean) (HitLocation :type Vector :default "0, 0, 0") (HitNormal :type Vector :default "0, 0, 0") (NormalImpulse :type Vector :default "0, 0, 0") (Hit :type Hit%20Result%20Structure%20%28by%20ref%29))
  (Development|PrintString (Utilities|GetDisplayName OtherComp)))

(fn ConstructionScript
  (bind _projectiledata (Variables|InitVars|GetProjectileData))
  (bind _projectilemovement (Variables|Default|GetProjectileMovement))
  (bind (_initiallspeed _maxspeed _projectilegracityscale) (Utilities|Struct|BreakS_Projectile _projectiledata))
  (Variables|/Script/Engine.ProjectileMovementComponent|SetInitialSpeed _projectilemovement _initiallspeed)
  (Variables|/Script/Engine.ProjectileMovementComponent|SetMaxSpeed _projectilemovement _maxspeed)
  (Variables|/Script/Engine.ProjectileMovementComponent|SetProjectileGravityScale _projectilemovement _projectilegracityscale))