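; Data-driven projectile actor that sets its movement, lifespan and mesh from ProjectileData and deals damage on impact.
; Sphere overlaps and hits broadcast OnProjectileHit and spawn impact Niagara; non-AOE overlaps also send direct damage through the target's damage component message.
; On blocking hits, AOE projectiles swap to a hidden overlap mesh as the damage volume.
; Impact VFX repeats on a timed loop, damaging actors overlapping the mesh each pulse, then destroys the actor.
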(event OnComponentHit(Sphere)
  (params (HitComponent :type Primitive%20Component%20Object%20Reference) (OtherActor :type Actor%20Object%20Reference) (OtherComp :type Primitive%20Component%20Object%20Reference) (NormalImpulse :type Vector :default "0, 0, 0") (Hit :type Hit%20Result%20Structure%20%28by%20ref%29))
  (Utilities|FlowControl|Sequence
    (:then_0
      (Default|CallOnProjectileHit OtherActor OtherComp NormalImpulse Hit)
      (Actor|SetLifeSpan 0.0))
    (:then_1
      (|UpdateAOE_SM))
    (:then_2
      (Utilities|ImpactVFX))))

(event OnComponentBeginOverlap(Sphere)
  (params (OverlappedComponent :type Primitive%20Component%20Object%20Reference) (OtherActor :type Actor%20Object%20Reference) (OtherComp :type Primitive%20Component%20Object%20Reference) (OtherBodyIndex :type Integer) (bFromSweep :type Boolean) (SweepResult :type Hit%20Result%20Structure%20%28by%20ref%29))
  (bind (_bblockinghit _binitialoverlap _time _distance _location _impactpoint _normal _impactnormal _physmat _hitactor _hitcomponent _hitbonename) (Collision|BreakHitResult SweepResult))
  (bind _colliderdata (Variables|Initialize|GetColliderData))
  (bind (_damageclass _rawdamage) (Utilities|Struct|BreakS_DamageColliderData _colliderdata))
  (if (Math|Boolean|ANDBoolean (!= self OtherActor) (!= OtherActor (Game|GetInstigator)) (!= (Utilities|GetClass self) (Utilities|GetClass OtherActor)))
    (Default|CallOnProjectileHit OtherActor OtherComp (Transformation|GetVelocity) SweepResult)
    (Utilities|ImpactVFX)
    (if (not (Utilities|Struct|BreakS_ProjectileData (Variables|Initialize|GetProjectileData)))
      (bind _bpc_dc (Class|BPIPawn|DCGetDamageComponent(Message) OtherActor))
      (Class|IDamage|ExecuteComplexDamage(Message) _bpc_dc _damageclass _rawdamage (Components|GetOwner) (Utilities|Struct|MakeS_HitData _bblockinghit _location _impactpoint _normal _impactnormal _hitactor _hitcomponent _hitbonename)))))

(event Custom|DeliverAOE
  (bind _colliderdata (Variables|Initialize|GetColliderData))
  (bind (_damageclass _rawdamage) (Utilities|Struct|BreakS_DamageColliderData _colliderdata))
  (for _array_element (Collision|GetOverlappingActors (Variables|Default|GetStaticMesh) 0 :!class /Script/Engine.PrimitiveComponent)
    (bind _bpc_dc (Class|BPIPawn|DCGetDamageComponent(Message) _array_element))
    (Class|IDamage|ExecuteComplexDamage(Message) _bpc_dc _damageclass _rawdamage (Components|GetOwner))))

(event Custom|RepeatVFX
  (params (NiagaraSystem :type Niagara%20Component%20Object%20Reference) (Delay :type Float%20%28single-precision%29) (Count :type Integer))
  (if (> Count 0)
    (Niagara|ResetSystem NiagaraSystem)
    (Niagara|ReinitializeSystem NiagaraSystem)
    (Utilities|ActivateAOE true)
    (Default|CallOnParticleRepeat)
    (Utilities|FlowControl|Delay Delay)
    (bind _result (Math|Integer|DecrementInt Count)
      (:%20%20
        (CallFunction|RepeatVFX NiagaraSystem Delay _result)))
    (else
      (Effects|Components|ParticleSystem|ReleasetoPool (Variables|Default|GetNS))
      (Actor|DestroyActor))))

(event EventBeginPlay
  (bind _projectiledata (Variables|Initialize|GetProjectileData))
  (bind (_initialspeed _isaoe _aoe_duration _projectile_sm _projectilert) (Utilities|Struct|BreakS_ProjectileData _projectiledata))
  (Utilities|SetStaticMesh _projectile_sm (Math|Transform|MakeTransform (.location _projectilert) (.rotation _projectilert) (.scale _projectilert))))

(fn ConstructionScript
  (bind _projectiledata (Variables|Initialize|GetProjectileData))
  (bind _projectilemovement (Variables|Default|GetProjectileMovement))
  (bind (_initialspeed _maxspeed _projectilegracityscale _lifespan) (Utilities|Struct|BreakS_ProjectileData _projectiledata))
  (Variables|/Script/Engine.ProjectileMovementComponent|SetInitialSpeed _projectilemovement _initialspeed)
  (Variables|/Script/Engine.ProjectileMovementComponent|SetMaxSpeed _projectilemovement (Math|Float|Max(Float) _initialspeed _maxspeed))
  (Variables|/Script/Engine.ProjectileMovementComponent|SetProjectileGravityScale _projectilemovement _projectilegracityscale)
  (Actor|SetLifeSpan _lifespan))