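; World weapon pickup actor driven by a weapon data asset, which supplies its mesh, pickup radius and prompt.
; Construction sets the mesh, BeginPlay adds physics and sizes the overlap sphere, and an invalid asset destroys the actor.
; Interacting while Idle equips the weapon into the isometric player's primary or secondary attack-component slot.
; An occupied slot swaps, so the actor becomes the replaced weapon; filling an empty slot destroys it.
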(event Custom|EquipWeapon
  (params (EquippingCharRef :type Isometric%20Player%20Object%20Reference))
  (bind _wda_weapon (Variables|Default|GetWDA_Weapon))
  (bind _bpc_attackcomponent (Variables|/Game/ProjectR/IsometricPlayer/IsometricPlayer.IsometricPlayer_C|GetBPC_AttackComponent EquippingCharRef))
  (bind _weaponslot (Variables|/Game/ProjectR/Systems/WeaponSystem/PDA_Weapon.PDA_Weapon_C|GetWeaponSlot _wda_weapon))
  (bind _returnvalue (Utilities|Select :Index _weaponslot :NewEnumerator0 0 :NewEnumerator1 1))
  (Utilities|IsValid (Default|GetWeaponinSlot _bpc_attackcomponent _returnvalue)
    (:Is%20Valid
      (bind _oldweapon (Default|ReplaceWeaponinSlot _bpc_attackcomponent _returnvalue _wda_weapon))
      (CallFunction|UpdateWeapon _oldweapon))
    (:Is%20Not%20Valid
      (bind _equipsuccess_ (Default|SetWeaponinSlot _bpc_attackcomponent _returnvalue _wda_weapon))
      (if _equipsuccess_
        (Actor|DestroyActor)))))

(event EventBeginPlay
  (CallFunction|UpdateWeapon (Variables|Default|GetWDA_Weapon)))

(event Collision|EventActorBeginOverlap
  (params (OtherActor :type Actor%20Object%20Reference)))

(event EventTick
  (params (DeltaSeconds :type Float%20%28single-precision%29)))

(fn ConstructionScript
  (CallFunction|UpdateWeaponMesh))

(fn UpdateWeapon
  (params (PDA_Weapon :type PDA%20Weapon%20Object%20Reference))
  (bind _output_get (Variables|Default|SetWDA_Weapon PDA_Weapon))
  (Utilities|IsValid _output_get
    (:Is%20Valid
      (Utilities|FlowControl|Sequence
        (:then_0
          (CallFunction|UpdateWeaponMesh))
        (:then_1
          (CallFunction|UpdateWeaponPhysics))))
    (:Is%20Not%20Valid
      (Actor|DestroyActor))))

(fn UpdateWeaponMesh
  (bind _wda_weapon (Variables|Default|GetWDA_Weapon)
    (:then
      (bind _returnvalue (Components|StaticMesh|SetStaticMesh (Variables|Default|GetStaticMesh) (Variables|/Game/ProjectR/Systems/WeaponSystem/PDA_Weapon.PDA_Weapon_C|GetWeaponMesh _wda_weapon)))
      (return _returnvalue))
    (:else
      (Actor|DestroyActor))))

(fn UpdateWeaponPhysics
  (bind _wda_weapon (Variables|Default|GetWDA_Weapon)
    (:then
      (Components|Sphere|SetSphereRadius (Variables|Default|GetSphereOverlap) (Math|Float|SelectFloat (Variables|/Game/ProjectR/Systems/WeaponSystem/PDA_Weapon.PDA_Weapon_C|GetPickupRadius _wda_weapon) 0.0 (Variables|/Game/ProjectR/Systems/WeaponSystem/PDA_Weapon.PDA_Weapon_C|GetCanPickup? _wda_weapon)) true)
      (bind _staticmesh (Variables|Default|GetStaticMesh)
        (:then
          (Physics|SetSimulatePhysics _staticmesh true))
        (:else)))
    (:else
      (Actor|DestroyActor))))

(fn BeginOverlap
  (params (OverlappedComponent :type Primitive%20Component%20Object%20Reference) (CallingActorRef :type Actor%20Object%20Reference))
  (bind _wda_weapon (Variables|Default|GetWDA_Weapon))
  (return self (Utilities|String|SelectString (Utilities|String|Append "Press 'F' to pickup " (Utilities|String|ToString(Name) (Variables|/Game/ProjectR/Systems/WeaponSystem/PDA_Weapon.PDA_Weapon_C|GetWeaponName _wda_weapon))) "" (Variables|/Game/ProjectR/Systems/WeaponSystem/PDA_Weapon.PDA_Weapon_C|GetCanPickup? _wda_weapon))))

(fn EndOverlap
  (params (OverlappedComponent :type Primitive%20Component%20Object%20Reference) (CallingActorRef :type Actor%20Object%20Reference))
  (return ""))

(fn Interact
  (params (InteractingActor :type Actor%20Object%20Reference) (Activate? :type Boolean))
  (bind _current_action_state (Class|BPIIso|GetActionState(Message) InteractingActor))
  (switch Utilities|FlowControl|Switch|SwitchonE_ActionState _current_action_state
    (:NewEnumerator0
      (bind _asisometric_player (Utilities|Casting|CastToIsometricPlayer InteractingActor))
      (CallFunction|EquipWeapon _asisometric_player)
      (return (Utilities|String|Append "Equipped " (Utilities|String|ToString(Name) (Variables|/Game/ProjectR/Systems/WeaponSystem/PDA_Weapon.PDA_Weapon_C|GetWeaponName (Variables|Default|GetWDA_Weapon))))))))