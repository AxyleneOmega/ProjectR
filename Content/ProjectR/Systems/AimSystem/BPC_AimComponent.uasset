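; Actor component that drives the owner's aiming from gamepad stick or mouse cursor, with optional, settings-driven aim assist.
; A looping timer resolves an aim point lerped toward the nearest candidate, line-traces pawns, then steers controller yaw.
; Candidates are either all BPI_AimTarget actors or overlaps from a runtime-generated Geometry Script cone that follows raw aim.
; Debug drawing and a key cycling assist modes support tuning.
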(event Custom|DisableAim
  ;[0 0 0] Debug Toggle Aim Assist
  (Utilities|Time|ClearandInvalidateTimerbyHandle (Variables|Default|GetAimAssistHandle))
  (Variables|/Script/Engine.CharacterMovementComponent|SetbOrientRotationToMovement (Getters|Protected|GetOwnerCMC) true))

(event Custom|IterateAimType
  ;[0 0 0] Debug Toggle Aim Assist
  (Utilities|FlowControl|MultiGate false true -1
    (:Out%200
      (bind _returnvalue (Utilities|Time|SetTimerbyFunctionName 0 "AimTrace" 0.016 true true))
      (Variables|Default|SetAimAssistHandle _returnvalue)
      (bind _returnvalue_2 (Class|CRGameUserSettings|GetCRGameUserSettings))
      (Class|CRGameUserSettings|SetIsAimAssistEnabled _returnvalue_2 true)
      (Variables|/Script/Engine.CharacterMovementComponent|SetbOrientRotationToMovement (Getters|Protected|GetOwnerCMC) false)
      (Variables|Default|SetAimAssistType 1))
    (:Out%201
      (Variables|Default|SetAimAssistType 0))
    (:Out%202
      (bind _returnvalue_3 (Class|CRGameUserSettings|GetCRGameUserSettings))
      (Class|CRGameUserSettings|SetIsAimAssistEnabled _returnvalue_3 false))
    (:Out%203
      (Utilities|Time|ClearandInvalidateTimerbyHandle (Variables|Default|GetAimAssistHandle))
      (Variables|/Script/Engine.CharacterMovementComponent|SetbOrientRotationToMovement (Getters|Protected|GetOwnerCMC) true))))

(event Custom|EnableAIm
  ;[0 0 0] Debug Toggle Aim Assist
  (Utilities|FlowControl|Sequence
    (:then_0
      (bind _returnvalue (Utilities|Time|SetTimerbyFunctionName 0 "AimTrace" 0.016 true true))
      (Variables|Default|SetAimAssistHandle _returnvalue)
      (bind _returnvalue_2 (Class|CRGameUserSettings|GetCRGameUserSettings))
      (Class|CRGameUserSettings|SetIsAimAssistEnabled _returnvalue_2 true)
      (Variables|/Script/Engine.CharacterMovementComponent|SetbOrientRotationToMovement (Getters|Protected|GetOwnerCMC) false)
      (Variables|Default|SetAimAssistType 1))
    (:then_1
      (Utilities|FlowControl|MultiGate false true -1) ; enters at Reset
    )))

(event Custom|ToggleAim
  (params (Enable? :type Boolean))
  ;[0 0 0] Debug Toggle Aim Assist
  (if Enable?
    (CallFunction|EnableAIm)
    (else
      (CallFunction|DisableAim))))

(event Custom|EnableAimComponent
  (params (Enable :type Boolean))
  (Development|PrintString (Utilities|String|Append "Aim Component : " (Utilities|String|ToString(Boolean) Enable)) true true "(R=0.000000,G=0.660000,B=1.000000,A=1.000000)" 5.0)
  (CallFunction|ToggleAim Enable)
  (Rendering|SetVisibility (Variables|Default|GetAimCone) Enable true))

(event Input|EnhancedActionEvents|EnhancedInputActionIA_Aim
  (params (ActionValue :type Vector%202D%20Structure) (ElapsedSeconds :type Float%20%28double-precision%29) (TriggeredSeconds :type Float%20%28double-precision%29) (InputAction :type Input%20Action%20Object%20Reference :default "/Game/ProjectR/Framework/Input/Actions/IA_Aim.IA_Aim"))
  (bind _returnvalue (Getters|Protected|GetOwnerLoc))
  (bind _returnvalue_2 (Getters|Protected|GetOwnerUp))
  (bind _returnvalue_3 (Getters|Protected|GetOwnerViewRotation))
  (bind _returnvalue_4 (* (.x ActionValue) -1.0))
  (bind _returnvalue_5 (Math|Vector|MakeVector _returnvalue_4 (.y ActionValue) 0.0))
  (bind _returnvalue_6 (Math|Vector|RotateVectorAroundAxis _returnvalue_5 (.yaw _returnvalue_3) _returnvalue_2))
  (bind _returnvalue_7 (* _returnvalue_6 1000))
  ;[0 0 0] Gamepad Aim
  (Rendering|Debug|DrawDebugLine :LineStart _returnvalue :LineEnd (+ _returnvalue _returnvalue_7) :Duration (Utilities|Time|GetWorldDeltaSeconds) :Thickness 2.0)
  (Variables|Default|SetbIsUsingGamepadLook true)
  (Variables|Default|SetRawAimRelativeLocation _returnvalue_7))

(event EventTick
  (params (DeltaSeconds :type Float%20%28single-precision%29))
  (Aim|UpdateAim)
  (Development|PrintString (Utilities|String|ToString(Text) (Utilities|Text|FormatText "Aim Assist Type: {AT} 
AimedActors: {AC} 
Gamepad?: {G}" (Utilities|String|SelectString "Distance Falloff" "Angular Lerp" (Math|Conversions|ToBoolean(Integer) (Variables|Default|GetAimAssistType))) (Utilities|Set|Length (Variables|Default|GetActors)) (Variables|Default|GetbIsUsingGamepadLook))) (Variables|Default|GetDebug%20Mode?) false "(R=0.000000,G=0.660000,B=1.000000,A=1.000000)" (Utilities|Time|GetWorldDeltaSeconds)))

(event EventBeginPlay
  (|SpawnAimCone&SetupCollisionParams)
  (|SetDyanmicMeshParams)
  (|BindEventsAimCone)
  (CallFunction|ToggleAim true))

(event Input|KeyboardEvents|DebugKeyG
  (params (Key :type Key%20Structure :default "None") (ActionValue :type Input%20Action%20Value%20Structure))
  ;[0 0 0] Debug Toggle Aim Assist
  (:Pressed
    (CallFunction|IterateAimType)))

(event Input|KeyboardEvents|AnyKey
  (params (Key :type Key%20Structure :default "None"))
  (:Pressed
    (if (Class|KismetInputLibrary|KeyIsMouseButton Key)
      (Variables|Default|SetbIsUsingGamepadLook (Class|KismetInputLibrary|KeyIsGamepadKey Key)))))

(fn UpdateAim
  (bind _aimcone (Variables|Default|GetAimCone)
    (:then
      (Transformation|SetWorldRotation _aimcone (Math|Rotator|MakeRotfromXZ (Variables|Default|GetRawAimRelativeLocation) (Getters|Protected|GetOwnerUp)) false false))
    (:else)))

(fn OnBeginOverlap
  (params (OverlappedComponent :type Primitive%20Component%20Object%20Reference) (OtherActor :type Actor%20Object%20Reference) (OtherComp :type Primitive%20Component%20Object%20Reference) (OtherBodyIndex :type Integer) (bFromSweep :type Boolean) (SweepResult :type Hit%20Result%20Structure%20%28by%20ref%29))
  (if (!= OtherActor (Components|GetOwner))
    (Utilities|Set|Add (Variables|Default|GetActors) OtherActor)
    (return)))

(fn OnEndOverlap
  (params (OverlappedComponent :type Primitive%20Component%20Object%20Reference) (OtherActor :type Actor%20Object%20Reference) (OtherComp :type Primitive%20Component%20Object%20Reference) (OtherBodyIndex :type Integer))
  (Utilities|Set|Remove (Variables|Default|GetActors) OtherActor))

(fn GetOwnerLoc
  (return (Transformation|GetActorLocation (Components|GetOwner))))

(fn GetOwnerUp
  (return (Transformation|GetActorUpVector (Components|GetOwner))))

(fn GetOwnerMeshForward
  (bind _meshforward (Class|BPIPawn|GetMeshForwardVector(Message) (Components|GetOwner)))
  (return _meshforward))

(fn GetOwnerViewRotation
  (bind _rotator (Class|BPIPawn|GetViewRelativeRotation(Message) (Components|GetOwner)))
  (return _rotator))

(fn AimTrace
  (bind _returnvalue (Game|GetPlayerController 0))
  (bind (_actors _valid) (Aim|GetValidActors))
  (bind _returnvalue_2 (Getters|Protected|GetOwnerLoc))
  (bind _returnvalue_3 (Getters|Protected|GetOwnerLoc))
  (bind (_hitresult _returnvalue_4) (Game|Player|GetHitResultUnderCursorbyChannel _returnvalue "TraceTypeQuery3" false))
  (if (Variables|Default|GetbIsUsingGamepadLook)
    _
    (elif (and _returnvalue_4 (== _returnvalue (Pawn|GetController (Variables|/Script/Engine.Actor|GetInstigator (Components|GetOwner)))))
      (Variables|Default|SetRawAimRelativeLocation (- (.ImpactPoint (Collision|BreakHitResult _hitresult)) (Getters|Protected|GetOwnerLoc)))
      (else
        (return))))
  (Utilities|FlowControl|Sequence
    (:then_0
      (LocalVariables|SetResolvedTargetPoint (+ (Variables|Default|GetRawAimRelativeLocation) (Getters|Protected|GetOwnerLoc)))
      (LocalVariables|SetHomingCheckRadius -1.0)
      (bind _returnvalue_5 (Class|CRGameUserSettings|GetCRGameUserSettings))
      (if (Class|CRGameUserSettings|GetIsAimAssistEnabled _returnvalue_5)
        (bind _returnvalue_6 (Class|CRGameUserSettings|GetCRGameUserSettings))
        (Utilities|FlowControl|Sequence
          (:then_0
            (|DebugArrowToNearestEnemy _valid (.NearestActor (|CalculateMDF&NearestActor _actors (Class|CRGameUserSettings|GetAimFalloffRadius _returnvalue_6) (+ (Variables|Default|GetRawAimRelativeLocation) (Getters|Protected|GetOwnerLoc)))) (.DebugPrint (|CalculateMDF&NearestActor _actors (Class|CRGameUserSettings|GetAimFalloffRadius _returnvalue_6) (+ (Variables|Default|GetRawAimRelativeLocation) (Getters|Protected|GetOwnerLoc)))))
            ;[1 0 0] Debug Draw Raw Aim Input
            (Rendering|Debug|DrawDebugArrow (Math|Vector|MakeVector (.x _returnvalue_2) (.y _returnvalue_2) (.z _returnvalue_2)) (Math|Vector|MakeVector (.X (Math|Vector|BreakVector (+ (Variables|Default|GetRawAimRelativeLocation) (Getters|Protected|GetOwnerLoc)))) (.Y (Math|Vector|BreakVector (+ (Variables|Default|GetRawAimRelativeLocation) (Getters|Protected|GetOwnerLoc)))) (.z _returnvalue_2)) 1.0 "(R=0.923397,G=1.000000,B=0.942548,A=1.000000)" (Utilities|Time|GetWorldDeltaSeconds) 1.0))
          (:then_1
            (if _valid
              (bind _returnvalue_7 (Class|CRGameUserSettings|GetCRGameUserSettings))
              (LocalVariables|SetResolvedTargetPoint (.LerpedAimPoint (|ResolveAimLerp (.NearestActor (|CalculateMDF&NearestActor _actors (Class|CRGameUserSettings|GetAimFalloffRadius _returnvalue_6) (+ (Variables|Default|GetRawAimRelativeLocation) (Getters|Protected|GetOwnerLoc)))) (Class|CRGameUserSettings|GetAimLerpStrength _returnvalue_7) (Class|CRGameUserSettings|GetAimFalloffRadius _returnvalue_7) (.MidpointDifferentialFactor (|CalculateMDF&NearestActor _actors (Class|CRGameUserSettings|GetAimFalloffRadius _returnvalue_6) (+ (Variables|Default|GetRawAimRelativeLocation) (Getters|Protected|GetOwnerLoc)))) (+ (Variables|Default|GetRawAimRelativeLocation) (Getters|Protected|GetOwnerLoc)))))
              (LocalVariables|SetHomingCheckRadius (.HamingCheckRadius (|ResolveAimLerp (.NearestActor (|CalculateMDF&NearestActor _actors (Class|CRGameUserSettings|GetAimFalloffRadius _returnvalue_6) (+ (Variables|Default|GetRawAimRelativeLocation) (Getters|Protected|GetOwnerLoc)))) (Class|CRGameUserSettings|GetAimLerpStrength _returnvalue_7) (Class|CRGameUserSettings|GetAimFalloffRadius _returnvalue_7) (.MidpointDifferentialFactor (|CalculateMDF&NearestActor _actors (Class|CRGameUserSettings|GetAimFalloffRadius _returnvalue_6) (+ (Variables|Default|GetRawAimRelativeLocation) (Getters|Protected|GetOwnerLoc)))) (+ (Variables|Default|GetRawAimRelativeLocation) (Getters|Protected|GetOwnerLoc))))))))))
    (:then_1
      (for _index (range (Math|Integer|SelectInt 0 -1 true) (Math|Integer|SelectInt 0 1 true))
        ;[0 0 0] Linetrace
        (bind _returnvalue_8 (Class|CRGameUserSettings|GetCRGameUserSettings))
        (bind _output_get (Variables|Default|SetResolvedTargetDirection (Class|KismetMathLibrary|VectorNormal2D (Math|Vector|RotateVectorAroundAxis (- (LocalVariables|GetResolvedTargetPoint) _returnvalue_3) (* _index 0.9) (Getters|Protected|GetOwnerUp)) 0.0001)))
        (bind (_outhits _returnvalue_9) (Class|KismetSystemLibrary|LineTraceMultiforObjects (Getters|Protected|GetOwnerLoc) (+ (* _output_get 3000) _returnvalue_3) (Utilities|Array|MakeArray "ObjectTypeQuery3") false 0 "ForOneFrame" true (Math|Color|SelectColor "(R=0.000000,G=1.000000,B=1.000000,A=1.000000)" "(R=1.000000,G=1.000000,B=0.000000,A=1.000000)" (Class|CRGameUserSettings|GetIsAimAssistEnabled _returnvalue_8)) (Math|Color|SelectColor "(R=0.000000,G=0.000000,B=1.000000,A=1.000000)" "(R=0.000000,G=1.000000,B=0.000000,A=1.000000)" (Class|CRGameUserSettings|GetIsAimAssistEnabled _returnvalue_8)) (Utilities|Time|GetWorldDeltaSeconds)))
        (if _returnvalue_9
          (LocalVariables|SetHitBoolean _returnvalue_9)
          (LocalVariables|SetHitResult (Utilities|Array|Get(acopy) _outhits))))
      (if (LocalVariables|GetHitBoolean)
        (bind _returnvalue_10 (Class|CRGameUserSettings|GetCRGameUserSettings))
        ;[0 0 0] Homing Target Check
        (Collision|SphereTraceForObjects (Math|Vector|SelectVector (.ImpactPoint (Collision|BreakHitResult (LocalVariables|GetHitResult))) (Math|Vector|MakeVector (.X (Math|Vector|BreakVector (LocalVariables|GetResolvedTargetPoint))) (.Y (Math|Vector|BreakVector (LocalVariables|GetResolvedTargetPoint))) (.Z (Math|Vector|BreakVector (Getters|Protected|GetOwnerLoc)))) true) (Math|Vector|SelectVector (.ImpactPoint (Collision|BreakHitResult (LocalVariables|GetHitResult))) (Math|Vector|MakeVector (.X (Math|Vector|BreakVector (LocalVariables|GetResolvedTargetPoint))) (.Y (Math|Vector|BreakVector (LocalVariables|GetResolvedTargetPoint))) (.Z (Math|Vector|BreakVector (Getters|Protected|GetOwnerLoc)))) true) (Math|Float|SelectFloat (Math|Float|SelectFloat (Math|Float|Max(Float) (.x (.BoxExtent (Collision|GetActorBounds (.HitActor (Collision|BreakHitResult (LocalVariables|GetHitResult))) true false))) (.y (.BoxExtent (Collision|GetActorBounds (.HitActor (Collision|BreakHitResult (LocalVariables|GetHitResult))) true false))) (.z (.BoxExtent (Collision|GetActorBounds (.HitActor (Collision|BreakHitResult (LocalVariables|GetHitResult))) true false)))) 0.0 (Utilities|DoesObjectImplementInterface (.HitActor (Collision|BreakHitResult (LocalVariables|GetHitResult))) "/Game/ProjectR/Enemies/BPI_AimTarget.BPI_AimTarget_C")) (LocalVariables|GetHomingCheckRadius) (< (LocalVariables|GetHomingCheckRadius) 0.0)) (Utilities|Array|MakeArray "ObjectTypeQuery3") false 0 "ForDuration" true (Math|Color|SelectColor "(R=0.000000,G=1.000000,B=1.000000,A=1.000000)" "(R=1.000000,G=1.000000,B=0.000000,A=1.000000)" (Class|CRGameUserSettings|GetIsAimAssistEnabled _returnvalue_10)) (Math|Color|SelectColor "(R=0.000000,G=0.000000,B=1.000000,A=1.000000)" "(R=0.000000,G=1.000000,B=0.000000,A=1.000000)" (Class|CRGameUserSettings|GetIsAimAssistEnabled _returnvalue_10)) (Utilities|Time|GetWorldDeltaSeconds))))
    (:then_2
      (Development|PrintString (Utilities|String|ToString(Vector) (Variables|Default|GetResolvedTargetDirection)) (Variables|Default|GetDebug%20Mode?) false "(R=1.000000,G=0.213901,B=0.313667,A=1.000000)" (Utilities|Time|GetWorldDeltaSeconds))
      (Pawn|Input|AddControllerYawInput (Variables|/Script/Engine.Actor|GetInstigator (Components|GetOwner)) (* (Class|KismetMathLibrary|VectorCosineAngle2D (Variables|Default|GetResolvedTargetDirection) (Math|Vector|NegateVector (Getters|Protected|GetOwnerMeshForward))) 1e+01))
      (return))))

(fn GetOwnerCMC
  (bind _cmc (Class|BPIPawn|GetCMC(Message) (Components|GetOwner)))
  (return _cmc))

(fn GetRawAimRL
  (return (Variables|Default|GetRawAimRelativeLocation)))

(fn GetResolvedAimDir
  (return (Variables|Default|GetResolvedTargetDirection)))

(fn GetAimStatus
  (bind _returnvalue (Class|CRGameUserSettings|GetCRGameUserSettings))
  (return (Class|CRGameUserSettings|GetIsAimAssistEnabled _returnvalue) (Utilities|Time|IsTimerActivebyHandle (Variables|Default|GetAimAssistHandle))))

(fn OnRepDebugMode?
  (Development|SetHiddeninGame (Variables|Default|GetAimCone) (not (Variables|Default|GetDebug%20Mode?)) true))

(fn GetValidActors
  (bind _actors (Variables|Default|GetActors))
  (if (Math|Conversions|ToBoolean(Integer) (Variables|Default|GetAimAssistType))
    (bind _outactors (Actor|GetAllActorswithInterface "/Game/ProjectR/Enemies/BPI_AimTarget.BPI_AimTarget_C"))
    (return _outactors (Utilities|Array|IsNotEmpty _outactors))
    (else
      (bind _result (Utilities|Set|ToArray _actors))
      (return _result (Utilities|Set|IsNotEmpty _actors)))))

(fn GetAimConeRef
  (return (Variables|Default|GetAimCone)))