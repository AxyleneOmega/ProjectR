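; Health component that handles damage, healing and death for its owning actor, broadcasting health-change and death events.
; StartSystem initialises health through a SetHealth chain of server and multicast events, while Damage and Heal clamp and write CurrentHealth directly, bypassing that chain.
; ExecuteComplexDamage async-loads and constructs a damage class, asks it for a response class, then loads and executes that response on the owner.
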(event Custom|Start%20System
  (params (Max%20Health :type Float%20%28double-precision%29))
  (bind _output_get (Variables|Default|SetMaxHealth Max%20Health))
  (CallFunction|SetHealth _output_get)
  (Default|CallOnHealthChange 0.0)
  (Variables|Default|SetisDead? false)
  (Variables|Default|SetcanTakeDamage true))

(event Custom|SetHealth
  (params (New%20Health :type Float%20%28double-precision%29))
  ;[1 0.2543 0.5426] Replicate Health
  (bind _output_get (Variables|Default|SetCurrentHealth New%20Health))
  (CallFunction|SetHealthSERVER _output_get))

(event Custom|SetHealth%20MULTI
  (params (New%20Health :type Float%20%28double-precision%29))
  ;[1 0.2543 0.5426] Replicate Health
  (Variables|Default|SetCurrentHealth New%20Health))

(event Custom|Set%20Health%20SERVER
  (params (New%20Health :type Float%20%28double-precision%29))
  ;[1 0.2543 0.5426] Replicate Health
  (bind _output_get (Variables|Default|SetCurrentHealth New%20Health))
  (CallFunction|SetHealthMULTI _output_get))

(event EventBeginPlay
  (Variables|Default|SetOwner%20Ref (Components|GetOwner)))

(event EventTick
  (params (DeltaSeconds :type Float%20%28single-precision%29)))

(event EventExecuteComplexDamage
  (params (DamageClass :type CR%20Class%20Damage%20Soft%20Class%20Reference) (RawAmount :type Float%20%28double-precision%29) (Instigator :type Actor%20Object%20Reference) (HitData :type S%20Hit%20Data%20Structure))
  (bind _returnvalue (Components|GetOwner))
  (Development|PrintString (Utilities|String|Append (Utilities|GetDisplayName _returnvalue) " : " (Utilities|String|ToString(Float) RawAmount)) true true "(R=1.000000,G=0.133333,B=0.155913,A=1.000000)")
  (bind _class (Utilities|AsyncLoadClassAsset DamageClass)
    (:Completed
      (bind _ascr_class_damage (Utilities|Casting|CastToCR_ClassDamageClass _class))
      (bind _returnvalue_2 (Game|ConstructObjectfromClass _returnvalue _ascr_class_damage))
      (bind _damageresponse (Default|TakeDamageResponseSpecific _returnvalue_2 RawAmount _returnvalue Instigator))
      (bind _class_2 (Utilities|AsyncLoadClassAsset _damageresponse)
        (:Completed
          (bind _ascr_damage_response (Utilities|Casting|CastToCR_DamageResponseClass _class_2))
          (bind _returnvalue_3 (Game|ConstructObjectfromClass _returnvalue _ascr_damage_response))
          (Default|DRExecuteDamageResponse _returnvalue_3 _returnvalue))))))

(fn Damage
  (params (Damage :type Float%20%28double-precision%29))
  (Development|PrintString "Simple Damage")
  (if (and (Variables|Default|GetcanTakeDamage) (not (Variables|Default|GetisDead?)))
    (Default|CallOnHealthChange (- (Math|Float|Clamp(Float) (- (Variables|Default|GetCurrentHealth) Damage) 0.0 (Variables|Default|GetMaxHealth)) (Variables|Default|GetCurrentHealth)))
    (bind _output_get (Variables|Default|SetCurrentHealth (Math|Float|Clamp(Float) (- (Variables|Default|GetCurrentHealth) Damage) 0.0 (Variables|Default|GetMaxHealth))))
    (if (<= _output_get 0.0)
      (Variables|Default|SetisDead? true)
      (Variables|Default|SetcanTakeDamage false)
      (Default|CallOnDeath)
      (return true 0.0)
      (else
        (return false (Variables|Default|GetCurrentHealth))))
    (else
      (return false (Variables|Default|GetCurrentHealth)))))

(fn GetCurrentHealth
  (return (Variables|Default|GetCurrentHealth)))

(fn GetHealthPercent
  (return (/ (Variables|Default|GetCurrentHealth) (Variables|Default|GetMaxHealth))))

(fn GetMaxHealth
  (return (Variables|Default|GetMaxHealth)))

(fn Heal
  (params (Heal%20Amount :type Float%20%28double-precision%29))
  (if (and (Variables|Default|GetcanHeal) (not (Variables|Default|GetisDead?)))
    (Default|CallOnHealthChange (- (Math|Float|Clamp(Float) (+ Heal%20Amount (Variables|Default|GetCurrentHealth)) 0.0 (Variables|Default|GetMaxHealth)) (Variables|Default|GetCurrentHealth)))
    (bind _output_get (Variables|Default|SetCurrentHealth (Math|Float|Clamp(Float) (+ Heal%20Amount (Variables|Default|GetCurrentHealth)) 0.0 (Variables|Default|GetMaxHealth))))
    (return _output_get)))