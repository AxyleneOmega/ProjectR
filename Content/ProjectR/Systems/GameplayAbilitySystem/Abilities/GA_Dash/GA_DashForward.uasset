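; GA_DashForward is a dash gameplay ability that pushes the avatar with a constant root motion force.
; On commit it loosens camera lag, fetches dash parameters from the avatar by interface message, and plays a montage rate-scaled to the dash duration.
; When the force finishes it ends the ability, then sets up a wait for the motion cooldown tag to interpolate camera lag back to a tighter speed.
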(event Ability|EventActivateAbility
  (bind _returnvalue (select false "/Game/ProjectR/Assets/Anims/Mobility/Dash/DashMontage.DashMontage" "/Game/ProjectR/Assets/Anims/Mobility/Dash/DashMontage.DashMontage"))
  (bind _returnvalue_2 (Ability|CommitAbility))
  (if _returnvalue_2
    (Class|BPIPawn|ConfigCameraLag(Message) (Ability|GetAvatarActorfromActorInfo) (Utilities|Struct|MakeF_CameraLagParams true 1e+01 0.0) true 0.01)
    (Utilities|FlowControl|Sequence
      (:then_0
        (bind (_worlddirection _strength _duration _bisadditive _strengthovertime _velocityonfinishmode _setvelocityonfinish _clampvelocityonfinish _benablegravity) (Class|BPIGameplayAbilities|GADashGetData(Message) (Ability|GetAvatarActorfromActorInfo)))
        (|PlayMontageandWaitProxy "DashMontage" _returnvalue (/ (Animation|GetPlayLength _returnvalue) _duration) "Default" true 1.0 0.0 false))
      (:then_1
        (Ability|Tasks|ApplyRootMotionConstantForce "DashForce" _worlddirection _strength _duration _bisadditive _strengthovertime _velocityonfinishmode _setvelocityonfinish _clampvelocityonfinish _benablegravity
          (:OnFinish
            (Utilities|FlowControl|Sequence
              (:then_0
                (Ability|EndAbility))
              (:then_1
                (Ability|Tasks|WaitGameplayTagAddToActor (Ability|GetAvatarActorfromActorInfo) "(TagName=\"Character.State.Action.Motion.Cooldown\")" true
                  (:Added
                    (Class|BPIPawn|ConfigCameraLag(Message) (Ability|GetAvatarActorfromActorInfo) (Utilities|Struct|MakeF_CameraLagParams true 1e+02 0.0) true (* _duration 3.0))))))))))
    (else
      (Ability|EndAbility))))

(event Ability|EventOnEndAbility
  (params (bWasCancelled :type Boolean))
  (if bWasCancelled
    _))