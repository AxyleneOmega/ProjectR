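; Attack component for IsometricPlayer that manages weapon slots, scrolling between two, and dropping weapons as BP_Weapon actors.
; Attack input goes to the active weapon, or to a default hand combo asset when the slot is empty.
; One runtime-added static mesh collider takes its mesh, socket, transform and damage from passed-in collider data, sending complex damage on overlap.
; It also spawns projectiles at the weapon socket and prints debug text.
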(event Custom|Attack
  (bind _active_slot (ActiveSlot|GetActiveSlot))
  (bind _slot_weapon (WeaponSlot|GetWeaponinSlot _active_slot))
  (Utilities|IsValid _slot_weapon
    (:Is%20Valid
      (Default|WeaponExecuteAttack _slot_weapon))
    (:Is%20Not%20Valid
      (Default|RecieveAttackInput (Variables|Default|GetDefaultHandComboDA) true "NewEnumerator0"))))

(event EventBeginPlay
  (bind _asisometric_player (Utilities|Casting|CastToIsometricPlayer (Components|GetOwner)))
  (bind _output_get (Variables|Refs|SetCharRef _asisometric_player))
  (|AttackColliderSetup _output_get)
  (Default|CallActiveSlotUpdated)
  (Default|SetCharacterRef (Variables|Default|GetDefaultHandComboDA) (Variables|Refs|GetCharRef)))

(event EventTick
  (params (DeltaSeconds :type Float%20%28single-precision%29))
  (bind _weaponslots (Variables|Runtime|GetWeaponSlots))
  (Development|PrintString (Utilities|String|Append "0] " (Utilities|GetDisplayName (Utilities|Array|Get(acopy) _weaponslots)) " 
1] " (Utilities|GetDisplayName (Utilities|Array|Get(acopy) _weaponslots 1)) " 
Collider SM :  " (Utilities|GetDisplayName (Variables|/Script/Engine.StaticMeshComponent|GetStaticMesh (Variables|Default|GetAttackCollider)))) true false "(R=0.320543,G=0.000000,B=1.000000,A=1.000000)" DeltaSeconds))

(fn GetWeaponinSlot
  (params (SlotNumber :type Integer))
  (return (Utilities|Array|Get(acopy) (Variables|Runtime|GetWeaponSlots) SlotNumber)))

(fn SetWeaponinSlot
  (params (SlotNumber :type Integer) (Weapon :type PDA%20Weapon%20Object%20Reference))
  (Utilities|Array|SetArrayElem (Variables|Runtime|GetWeaponSlots) SlotNumber Weapon true)
  (ActiveSlot|ChangeActiveSlot SlotNumber)
  (Default|CallWeaponSlotUpdated SlotNumber Weapon)
  (Utilities|IsValid Weapon
    (:Is%20Valid
      (Default|SetWeaponOwner Weapon (Variables|Refs|GetCharRef)))
    (:Is%20Not%20Valid
      _))
  (return true))

(fn ReplaceWeaponinSlot
  (params (SlotNumber :type Integer) (NewWeapon :type PDA%20Weapon%20Object%20Reference))
  (LocalVariables|SetTempWeapon (WeaponSlot|GetWeaponinSlot SlotNumber))
  (bind _equipsuccess_ (WeaponSlot|SetWeaponinSlot SlotNumber NewWeapon))
  (if _equipsuccess_
    (return (LocalVariables|GetTempWeapon))
    (else
      (return 0))))

(fn GetActiveSlot
  (return (Variables|Runtime|GetActiveSlot)))

(fn ChangeActiveSlot
  (params (New%20Active%20Slot :type Integer))
  (bind _output_get (Variables|Runtime|SetActiveSlot New%20Active%20Slot))
  (Default|CallActiveSlotUpdated _output_get))

(fn DropWeapon
  (bind _activeslot (Variables|Runtime|GetActiveSlot))
  (bind _charref (Variables|Refs|GetCharRef))
  (bind _slot_weapon (WeaponSlot|GetWeaponinSlot _activeslot))
  (Utilities|IsValid _slot_weapon
    (:Is%20Valid
      (LocalVariables|SetWeaponName (Variables|/Game/ProjectR/Systems/WeaponSystem/PDA_Weapon.PDA_Weapon_C|GetWeaponName _slot_weapon))
      (Game|SpawnActorfromClass "/Game/ProjectR/Systems/WeaponSystem/BP_Weapon.BP_Weapon_C" (Math|Transform|MakeTransform (Transformation|GetActorLocation _charref) "0, 0, 0" "1.000000,1.000000,1.000000") "AdjustIfPossibleButAlwaysSpawn" "MultiplyWithRoot" 0 _slot_weapon _charref)
      (WeaponSlot|SetWeaponinSlot _activeslot)
      (return (Utilities|String|Append "Dropped " (Utilities|String|ToString(Name) (LocalVariables|GetWeaponName)))))
    (:Is%20Not%20Valid
      (return ""))))

(fn GetCurrentlyEquippedWeapon
  (return (WeaponSlot|GetWeaponinSlot (ActiveSlot|GetActiveSlot))))

(fn ScrollActiveSlot
  (params (Scroll%20Value :type Float%20%28double-precision%29))
  (ActiveSlot|ChangeActiveSlot (Math|Integer|%(Integer) (+ (ActiveSlot|GetActiveSlot) (Math|Integer|SelectInt 1 (+ -1 (Class|KismetSystemLibrary|MakeLiteralInteger 2)) (Math|Conversions|ToBoolean(Integer) (Math|Float|Truncate (/ (+ Scroll%20Value 1.0) 2.0))))) 2)))

(fn UpdateCanCombo
  (params (Enable :type Boolean))
  (bind _active_slot (ActiveSlot|GetActiveSlot))
  (bind _slot_weapon (WeaponSlot|GetWeaponinSlot _active_slot))
  (Utilities|IsValid _slot_weapon
    (:Is%20Valid
      (Default|SetIsWeaponComboEnabled _slot_weapon Enable))))

(fn ActivateCollider
  (bind _attackcollider (Variables|Default|GetAttackCollider))
  (Components|Activation|Activate _attackcollider false)
  (Collision|SetCollisionEnabled _attackcollider "QueryAndProbe")
  (Development|PrintString "ActivatedCollider"))

(fn DeactivateCollider
  (bind _attackcollider (Variables|Default|GetAttackCollider))
  (Components|StaticMesh|SetStaticMesh _attackcollider 0)
  (Components|Activation|Deactivate _attackcollider)
  (Variables|Runtime|SetCurrentDamageClass 0)
  (Variables|Runtime|SetCurrentDamage 0.0)
  (Development|PrintString "Deactivated Collidor"))

(fn GetWeaponSocketName
  (bind _active_slot (ActiveSlot|GetActiveSlot))
  (bind _slot_weapon (WeaponSlot|GetWeaponinSlot _active_slot))
  (Utilities|IsValid _slot_weapon
    (:Is%20Valid
      (return (Variables|/Game/ProjectR/Systems/WeaponSystem/PDA_Weapon.PDA_Weapon_C|GetSocketAttachName _slot_weapon)))
    (:Is%20Not%20Valid
      (return "hand_l"))))

(fn ColliderUpdateData
  (params (ColliderSM :type S%20Damage%20Collider%20Data%20Structure))
  (bind _attackcollider (Variables|Default|GetAttackCollider))
  (Variables|Runtime|SetCurrentDamageClass (.damageclass ColliderSM))
  (Variables|Runtime|SetCurrentDamage (.rawdamage ColliderSM))
  (|AttachComponent _attackcollider (.socketoverride ColliderSM))
  (|RelativeTransformComponent _attackcollider (.colliderrelativetransform ColliderSM) "0, 0, 0" "0, 0, 0" "0, 0, 0")
  (Components|StaticMesh|SetStaticMesh _attackcollider (.collidersm ColliderSM)))

(fn AttackColliderBeginOverlap
  (params (OverlappedComponent :type Primitive%20Component%20Object%20Reference) (OtherActor :type Actor%20Object%20Reference) (OtherComp :type Primitive%20Component%20Object%20Reference) (OtherBodyIndex :type Integer) (bFromSweep :type Boolean) (SweepResult :type Hit%20Result%20Structure%20%28by%20ref%29))
  (bind _attackcollider (Variables|Default|GetAttackCollider))
  (bind _returnvalue (Components|GetOwner _attackcollider))
  (if (!= _returnvalue OtherActor)
    (Class|IDamage|ExecuteComplexDamage(Message) OtherActor (Utilities|ResolveSoftReference (Variables|Runtime|GetCurrentDamageClass)) (Variables|Runtime|GetCurrentDamage) _returnvalue (Utilities|Struct|MakeS_HitData (.bblockinghit SweepResult) (.location SweepResult) (.impactpoint SweepResult) (.normal SweepResult) (.impactnormal SweepResult) (.hitactor SweepResult) (.hitcomponent SweepResult) (.hitbonename SweepResult)))
    (Development|PrintString (Utilities|String|Append "AC Damage : " (Utilities|GetDisplayName OtherActor)) true true "(R=1.000000,G=0.000000,B=0.000000,A=1.000000)")
    (return)))

(fn AttackColliderEndOverlap
  (params (OverlappedComponent :type Primitive%20Component%20Object%20Reference) (OtherActor :type Actor%20Object%20Reference) (OtherComp :type Primitive%20Component%20Object%20Reference) (OtherBodyIndex :type Integer)))

(fn GetAttackCollider
  (return (Variables|Default|GetAttackCollider)))

(fn CancelCombo
  (bind _active_slot (ActiveSlot|GetActiveSlot))
  (bind _slot_weapon (WeaponSlot|GetWeaponinSlot _active_slot))
  (Utilities|IsValid _slot_weapon
    (:Is%20Valid
      (Default|CancelCombo _slot_weapon))))

(fn GetSocketWorldLoc
  (return (Transformation|GetSocketTransform (Variables|/Script/Engine.Character|GetMesh (Variables|Refs|GetCharRef)) (AttackCollider|GetWeaponSocketName) "RTS_World")))

(fn SpawnProjectile
  (params (Collider%20Data :type S%20Damage%20Collider%20Data%20Structure) (ProjectileData :type S%20Projectile%20Structure))
  (bind _returnvalue (AttackCollider|GetSocketWorldLoc))
  (bind _returnvalue_2 (Game|SpawnActorfromClass "/Game/ProjectR/Systems/WeaponSystem/BP_Projectile.BP_Projectile_C" (Math|Transform|MakeTransform (.location _returnvalue) (.rotation _returnvalue) "1.000000,1.000000,1.000000") "AlwaysSpawn" "MultiplyWithRoot" 0 Collider%20Data ProjectileData (Variables|Refs|GetCharRef)))
  (return _returnvalue_2))